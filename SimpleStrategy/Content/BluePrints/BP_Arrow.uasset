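; BP_Arrow is a projectile actor that flies toward an enemy location and destroys itself on touching the ground.
; Each Tick moves it without sweep along the unnormalized vector to LocationEnemy, scaled by Speed and delta time, so it slows as it nears the target.
; LocationEnemy is not set within this Blueprint.
; The Sphere overlap destroys the arrow only for actors tagged Ground, with no damage logic.
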(event `self.ReceiveBeginPlay`
  (set `self.Speed` 1.0)
  (set `self.CurrentLocation` (`self.StartLocationArrow`)))

(event `self.ReceiveTick`
  (params (DeltaSeconds :type "Float (single-precision)"))
  (set `self.CurrentLocation` (`self.K2_GetActorLocation`))
  (set `self.Direction` (- (`self.LocationEnemy`) (`self.CurrentLocation`)))
  (`self.K2_SetActorLocation` (+ (`self.CurrentLocation`) (* (* DeltaSeconds (`self.Speed`)) (`self.Direction`)))))

(event `self.Sphere.OnComponentBeginOverlap`
  (params (OverlappedComponent :type "PrimitiveComponent Object Reference") (OtherActor :type "Actor Object Reference") (OtherComp :type "PrimitiveComponent Object Reference") (OtherBodyIndex :type Integer) (bFromSweep :type Boolean) (SweepResult :type "HitResult Structure (by ref)"))
  (if (`self.ActorHasTag` OtherActor "Ground")
    (`self.K2_DestroyActor`)))

(fn `UserConstructionScript`
  (set `self.StartLocationArrow` (`self.K2_GetActorLocation` self)))