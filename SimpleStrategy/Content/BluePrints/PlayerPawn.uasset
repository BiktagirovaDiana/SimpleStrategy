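; Player pawn with an orbit camera on a spring arm, plus zoom and directional movement.
; Construction sets default angles and limits and moves OrbitPivot to the last BP_SpawnOrbitPivot found.
; While Orbit is held, Turn accumulates yaw and rotates the arm, while LookUp sets clamped pitch from the current input without accumulating it.
; Zoom adjusts arm length within limits, and move axes add input along actor forward and right vectors.
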(event `self.ReceiveBeginPlay`)

(event `InputAction|Orbit`
  (params (Key :type "Key Structure"))
  (bind _returnvalue (`GameplayStatics.GetPlayerController` 0))
  (:`Pressed`
    (set `self.IsOrbiting` true)
    (set `PlayerController.bShowMouseCursor` true _returnvalue))
  (:`Released`
    (set `self.IsOrbiting` false)
    (set `PlayerController.bShowMouseCursor` true _returnvalue)))

(event `InputAxis|Turn`
  (params (AxisValue :type "Float (single-precision)"))
  (if (`self.IsOrbiting`)
    (set `self.Yaw` (+ (`self.Yaw`) (* (`self.GetInputAxisValue`) (`self.Sensitivity`) 100.0)))
    (`SceneComponent.K2_SetWorldRotation` (`self.SpringArm`) (`KismetMathLibrary.MakeRotator` 0.0 (`self.Pitch`) (`self.Yaw`)) false false)))

(event `InputAxis|LookUp`
  (params (AxisValue :type "Float (single-precision)"))
  (if (`self.IsOrbiting`)
    (set `self.Pitch` (`KismetMathLibrary.FClamp` (* (`self.GetInputAxisValue`) (`self.Sensitivity`) 100.0) (`self.PitchMin`) (`self.PitchMax`)))))

(event `InputAxis|Zoom`
  (params (AxisValue :type "Float (single-precision)"))
  (bind _output_get (set `self.CurrentLenght` (- (`SpringArmComponent.TargetArmLength` (`self.SpringArm`)) (* AxisValue 250.0))))
  (set `SpringArmComponent.TargetArmLength` (`KismetMathLibrary.FClamp` _output_get 1000.0 6000.0) (`self.SpringArm`)))

(event `InputAxis|MoveForward`
  (params (AxisValue :type "Float (single-precision)"))
  (`self.AddMovementInput` (`self.GetActorForwardVector`) AxisValue))

(event `InputAxis|MoveRight`
  (params (AxisValue :type "Float (single-precision)"))
  (`self.AddMovementInput` (`self.GetActorRightVector`) AxisValue))

(fn `UserConstructionScript`
  (bind _outactors (`GameplayStatics.GetAllActorsOfClass` "/Game/BluePrints/BP_SpawnOrbitPivot.BP_SpawnOrbitPivot_C"))
  (for _array_element _outactors
    _)
  (`SceneComponent.K2_SetWorldLocation` (`self.OrbitPivot`) (`self.K2_GetActorLocation` _array_element) false false)
  (set `self.IsOrbiting` false)
  (set `self.Yaw` 0.0)
  (set `self.Pitch` -45.0)
  (set `self.Sensitivity` 0.05)
  (set `self.PitchMin` -80.0)
  (set `self.PitchMax` -10.0))