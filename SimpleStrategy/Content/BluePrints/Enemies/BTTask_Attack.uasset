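; Behavior tree task that makes an enemy AI attack the building stored in its TargetActor blackboard key.
; Its tick accumulates time and, about once per second, casts the target to BP_BaseBuild and calls DamageBuild.
; When the building's HP equals zero, the task finishes as failed, its only exit.
; A failed cast just prints a debug string and leaves the task running.
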(event `self.ReceiveExecuteAI`
  (params (OwnerController :type "AIController Object Reference") (ControlledPawn :type "Pawn Object Reference")))

(event `self.ReceiveTickAI`
  (params (OwnerController :type "AIController Object Reference") (ControlledPawn :type "Pawn Object Reference") (DeltaSeconds :type "Float (single-precision)"))
  (bind _output_get (set `self.Timer` (+ DeltaSeconds (`self.Timer`))))
  (if (>= _output_get 1.0)
    (set `self.Timer` 0.0)
    (bind _asbp_base_build (cast `/Game/BluePrints/Builds/BP_BaseBuild` (`BTFunctionLibrary.GetBlackboardValueAsObject` (`self.TargetActor`)))
      (:`then`
        (`/Game/BluePrints/Builds/BP_BaseBuild.DamageBuild` _asbp_base_build)
        (if (== (`/Game/BluePrints/Builds/BP_BaseBuild.HP` _asbp_base_build) 0)
          (`self.FinishExecute` false)))
      (:`CastFailed`
        (`KismetSystemLibrary.PrintString` "Лошара")))))