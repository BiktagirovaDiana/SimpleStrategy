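; Clickable building plot for a strategy game that lets the player place one structure while the plot is free.
; A click opens a WBP_Builds widget that receives the plot; BuyBuild spawns the indexed class from BPBuilds at PointSpawn and marks it occupied.
; When an actor leaves the Box, IsFree is set to whether that actor has the "Building" tag.
; It caches StrategyGameMode's resources widget and exposes an insufficient-resources message, without checking costs itself.
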(event `self.ReceiveBeginPlay`
  (set `self.SpawnPoint` (`KismetMathLibrary.Conv_VectorToTransform` (`SceneComponent.K2_GetComponentLocation` (`self.PointSpawn`))))
  (set `self.isFree` true)
  (add `self.OnClicked` (delegate `OnClicked_Event`))
  (bind _asstrategy_game_mode (cast `/Game/BluePrints/StrategyGameMode` (`GameplayStatics.GetGameMode`))
    (:`then`
      (bind _output_get (set `self.GameMode` _asstrategy_game_mode))
      (set `self.WBP_Resources` (`/Game/BluePrints/StrategyGameMode.WBP_Resources` _output_get))
      (set `self.Plot` self))
    (:`CastFailed`
      (`KismetSystemLibrary.PrintString` "Cast на GameMode не сработан"))))

(event `PrintResources`
  (`KismetSystemLibrary.PrintString` "НЕДОСТАТОЧНО РЕСУРСОВ" true true (struct :`R` 1.0 :`B` 0.050343 :`A` 1.0)))

(event `OnClicked_Event` :!signature `self.OnClicked`
  (params (TouchedActor :type "Actor Object Reference") (ButtonPressed :type "Key Structure" :default "None"))
  (if (`self.isFree`)
    (bind _returnvalue (`|CreateWidget` "/Game/Blueprints/UI/WBP_Builds.WBP_Builds_C" null (`self.Plot`)))
    (bind _output_get (set `self.WBP_Builds` _returnvalue))
    (`UserWidget.AddToViewport` _output_get 0)))

(event `BuyBuild`
  (params (IndexBuild :type "Float (double-precision)"))
  (if (`self.isFree`)
    (`|SpawnActorFromClass` (`|GetArrayItem` (`self.BP_Builds`) (`KismetMathLibrary.FTrunc` IndexBuild)) (`self.SpawnPoint`) "Undefined" "MultiplyWithRoot" null null)
    (set `self.isFree` false)
    (`KismetSystemLibrary.PrintString` "Постройка построена")))

(event `self.Box.OnComponentEndOverlap`
  (params (OverlappedComponent :type "PrimitiveComponent Object Reference") (OtherActor :type "Actor Object Reference") (OtherComp :type "PrimitiveComponent Object Reference") (OtherBodyIndex :type Integer))
  (set `self.isFree` (`self.ActorHasTag` OtherActor "Building")))

(fn `UserConstructionScript`)