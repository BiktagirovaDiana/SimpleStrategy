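; BP_KnightBase is the base knight unit, with hit points shown on an attached info widget.
; On BeginPlay it sets its starting HP and caches the WBP_KnightInfo widget from its widget component.
; DamageUnit removes one HP and refreshes the widget text; at zero it decrements the local knight count on its casern (BPCasern) and destroys the actor.
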(event `self.ReceiveBeginPlay`
  (set `self.Hp` 5)
  (bind _aswbp_knight_info (cast `/Game/BluePrints/UI/WBP_KnightInfo` (`WidgetComponent.GetUserWidgetObject` (`self.WidgetInfo`))))
  (bind _output_get (set `self.WBP_KnightInfo` _aswbp_knight_info))
  (`/Game/BluePrints/UI/WBP_KnightInfo.UpdateText` _output_get (`self.Hp`)))

(event `DamageUnit`
  (bind _output_get (set `self.Hp` (- (`self.Hp`) 1)))
  (`/Game/BluePrints/UI/WBP_KnightInfo.UpdateText` (`self.WBP_KnightInfo`) _output_get)
  (if (== (`self.Hp`) 0)
    (set `/Game/BluePrints/Builds/BP_Casern.LocalNumberKnight` (- (`/Game/BluePrints/Builds/BP_Casern.LocalNumberKnight` (`self.BP_Casern`)) 1) (`self.BP_Casern`))
    (`self.DestroyUnit`)))

(event `DestroyUnit`
  (`self.K2_DestroyActor`))

(fn `UserConstructionScript`)