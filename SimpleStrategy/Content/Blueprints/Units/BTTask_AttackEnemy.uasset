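; Behavior Tree task that makes a unit repeatedly attack the enemy knight stored in its TargetActor blackboard key.
; Each AI tick accumulates time and, once per second, casts the target to BP_EnemyKnight and calls DamageEnemy on it.
; When the knight's Hp reaches zero, the task finishes as failed; otherwise it keeps running.
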(event `self.ReceiveTickAI`
  (params (OwnerController :type "AIController Object Reference") (ControlledPawn :type "Pawn Object Reference") (DeltaSeconds :type "Float (single-precision)"))
  (set `self.DamageInterval` 1.0)
  (set `self.Timer` (+ DeltaSeconds (`self.Timer`)))
  (if (>= (`self.Timer`) (`self.DamageInterval`))
    (set `self.Timer` 0.0)
    (bind _asbp_enemy_knight (cast `/Game/Blueprints/Units/BP_EnemyKnight` (`BTFunctionLibrary.GetBlackboardValueAsObject` (`self.TargetActor`))))
    (`/Game/Blueprints/Units/BP_EnemyKnight.DamageEnemy` _asbp_enemy_knight)
    (if (== (`/Game/Blueprints/Units/BP_EnemyKnight.Hp` _asbp_enemy_knight) 0)
      (`self.FinishExecute` false))))