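; BP_EnemyKnight is an enemy knight unit that reads its starting HP from the DT_Enemy data table and shows it on an info widget.
; Arrows entering its arrow radius are destroyed and each costs one HP, updating the widget and destroying the knight at zero.
; A BP_KnightBase entering its unit radius notifies the enemy AI controller, cached on possession, that it is attacked.
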(event `self.ReceivePossessed`
  (params (NewController :type "Controller Object Reference"))
  (bind _asbp_ai_enemy_base (cast `/Game/BluePrints/Units/BP_AI_EnemyBase` (`AIBlueprintHelperLibrary.GetAIController` NewController)))
  (set `self.AI Controller` _asbp_ai_enemy_base))

(event `self.ReceiveBeginPlay`
  (`self.InitializationHP`)
  (bind _aswbp_enemy_info (cast `/Game/BluePrints/UI/WBP_EnemyInfo` (`WidgetComponent.GetUserWidgetObject` (`self.WidgetInfo`))))
  (bind _output_get (set `self.WBP_EnemyInfo` _aswbp_enemy_info))
  (`/Game/BluePrints/UI/WBP_EnemyInfo.UpdateText` _output_get (`self.Hp`))
  (set `self.Key Name` "IsAttacked"))

(event `self.ReceiveTick`
  (params (DeltaSeconds :type "Float (single-precision)")))

(event `DamageEnemy`
  (bind _output_get (set `self.Hp` (- (`self.Hp`) 1)))
  (`/Game/BluePrints/UI/WBP_EnemyInfo.UpdateText` (`self.WBP_EnemyInfo`) _output_get)
  (if (== (`self.Hp`) 0)
    (`self.DestroyEnemy`)))

(event `DestroyEnemy`
  (`self.K2_DestroyActor`))

(event `self.RadiusArrow.OnComponentBeginOverlap`
  (params (OverlappedComponent :type "PrimitiveComponent Object Reference") (OtherActor :type "Actor Object Reference") (OtherComp :type "PrimitiveComponent Object Reference") (OtherBodyIndex :type Integer) (bFromSweep :type Boolean) (SweepResult :type "HitResult Structure (by ref)"))
  (bind _asbp_arrow (cast `/Game/BluePrints/BP_Arrow` OtherActor))
  (`self.K2_DestroyActor` _asbp_arrow)
  (`self.DamageEnemy`))

(event `self.RadiusUnits.OnComponentBeginOverlap`
  (params (OverlappedComponent :type "PrimitiveComponent Object Reference") (OtherActor :type "Actor Object Reference") (OtherComp :type "PrimitiveComponent Object Reference") (OtherBodyIndex :type Integer) (bFromSweep :type Boolean) (SweepResult :type "HitResult Structure (by ref)"))
  (cast `/Game/BluePrints/Units/BP_KnightBase` OtherActor)
  (`/Game/BluePrints/Units/BP_AI_EnemyBase.Attacked` (`self.AI Controller`)))

(fn `InitializationHP`
  (bind _returnvalue (`|GetDataTableRow` "/Game/BluePrints/Units/DT_Enemy.DT_Enemy" "Knight")
    (:`then`
      (set `self.Hp` (`.HP_5_39590C704BC5C6F88A060EAA5CB4EA78` (break `/Game/BluePrints/Units/STR_EnemyData` _returnvalue))))))

(fn `UserConstructionScript`)