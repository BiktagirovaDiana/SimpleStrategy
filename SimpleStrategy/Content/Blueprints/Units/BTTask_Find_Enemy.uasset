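; Behavior tree task that finds the closest actor tagged "Enemy" to the AI-controlled pawn.
; On execute it scans all tagged actors, keeping the nearest within a fixed starting range.
; Each closer candidate overwrites the TargetLocation and TargetActor blackboard keys and calls FinishExecute with success inside the loop.
; When no actor is in range, the task never calls FinishExecute.
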(event `self.ReceiveExecuteAI`
  (params (OwnerController :type "AIController Object Reference") (ControlledPawn :type "Pawn Object Reference"))
  (set `self.MinDistance` 10000.0)
  (bind _outactors (`GameplayStatics.GetAllActorsWithTag` "Enemy"))
  (for _array_element _outactors
    (bind _returnvalue (`KismetMathLibrary.Vector_Distance` (`Actor.K2_GetActorLocation` _array_element) (`Actor.K2_GetActorLocation` ControlledPawn)))
    (if (< _returnvalue (`self.MinDistance`))
      (set `self.MinDistance` _returnvalue)
      (bind _output_get (set `self.ClosestActor` _array_element))
      (`BTFunctionLibrary.SetBlackboardValueAsVector` (`self.TargetLocation`) (`Actor.K2_GetActorLocation` _output_get))
      (`BTFunctionLibrary.SetBlackboardValueAsObject` (`self.TargetActor`) (`self.ClosestActor`))
      (`self.FinishExecute` true))))