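; Behavior tree task that points an enemy knight at the nearest actor tagged "Building".
; On execute it clears the knight's IsAttack flag, then scans the tagged actors for the shortest distance to the pawn.
; Each closer candidate is written to the TargetLocation and TargetActor blackboard keys.
; FinishExecute(true) fires inside the loop on each improvement, so the task never finishes when no building qualifies.
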(event `self.ReceiveExecuteAI`
  (params (OwnerController :type "AIController Object Reference") (ControlledPawn :type "Pawn Object Reference"))
  (bind _asbp_enemy_knight (cast `/Game/Blueprints/Units/BP_EnemyKnight` ControlledPawn))
  (set `/Game/Blueprints/Units/BP_EnemyKnight.isAttack` false _asbp_enemy_knight)
  (set `self.MinDistance` 1000000.0)
  (bind _outactors (`GameplayStatics.GetAllActorsWithTag` "Building"))
  (for _array_element _outactors
    (bind _returnvalue (`KismetMathLibrary.Vector_Distance` (`Actor.K2_GetActorLocation` _array_element) (`Actor.K2_GetActorLocation` ControlledPawn)))
    (if (< _returnvalue (`self.MinDistance`))
      (set `self.MinDistance` _returnvalue)
      (bind _output_get (set `self.ClosestActor` _array_element))
      (`BTFunctionLibrary.SetBlackboardValueAsVector` (`self.TargetLocation`) (`Actor.K2_GetActorLocation` _output_get))
      (`BTFunctionLibrary.SetBlackboardValueAsObject` (`self.TargetActor`) (`self.ClosestActor`))
      (`self.FinishExecute` true))))