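; Game mode for a day-based strategy game that creates the menu and HUD widgets and runs each battle.
; StartBattle reads the current day's enemy count from the level data table, then timer-driven events spawn knights at the spawners' average location.
; A repeating check calls Lose when no "Building" actors remain, or Win when no "Enemy" actors remain.
; Win advances the day and clears units; Lose pauses, though its widget variable is never assigned.
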(event `self.ReceiveBeginPlay`
  (bind _returnvalue (`|CreateWidget` "/Game/BluePrints/UI/WBP_MainMenu.WBP_MainMenu_C"))
  (`UserWidget.AddToViewport` _returnvalue 0)
  (bind _asbp_game_instance (cast `/Game/BluePrints/BP_GameInstance` (`GameplayStatics.GetGameInstance`))
    (:`then`
      (set `self.GameInstance` _asbp_game_instance))
    (:`CastFailed`
      (`KismetSystemLibrary.PrintString` "Каст не получен"))))

(event `StartGame`
  (`GameplayStatics.PlaySound2D` "/Game/Sounds/Ambient_Birds_Loop_04.Ambient_Birds_Loop_04" 1.0 1.0 0.0 null null)
  (bind _returnvalue (`|CreateWidget` "/Game/Blueprints/UI/WBP_Resources.WBP_Resources_C"))
  (`UserWidget.AddToViewport` _returnvalue 0)
  (bind _aswbp_resources (cast `/Game/Blueprints/UI/WBP_Resources` _returnvalue)
    (:`then`
      (bind _output_get (set `self.WBP_Resources` _aswbp_resources))
      (`/Game/Blueprints/UI/WBP_Resources.UpdateGoldText` _output_get)
      (bind _returnvalue_2 (`|CreateWidget` "/Game/BluePrints/UI/WBP_GameControl.WBP_GameControl_C"))
      (bind _output_get_2 (set `self.WBP_GameControl` _returnvalue_2))
      (`UserWidget.AddToViewport` _output_get_2 0)
      (`/Game/BluePrints/UI/WBP_GameControl.UpdateDailyIncomeText` (`self.WBP_GameControl`))
      (bind _outactors (`GameplayStatics.GetAllActorsOfClass` "/Game/BluePrints/Units/SpawnerEnemies.SpawnerEnemies_C"))
      (bind _returnvalue_3 (`GameplayStatics.GetActorArrayAverageLocation` _outactors))
      (set `self.LocationSpawners` (`|MakeArray` _returnvalue_3))
      (`|CreateWidget` "/Game/BluePrints/UI/WBP_Lose.WBP_Lose_C"))
    (:`CastFailed`
      (`KismetSystemLibrary.PrintString` "Cast не прочитан"))))

(event `UpdateGoldText`
  (`/Game/Blueprints/UI/WBP_Resources.UpdateGoldText` (`self.WBP_Resources`)))

(event `StartBattle`
  (bind _returnvalue (`|GetDataTableRow` (`/Game/BluePrints/BP_GameInstance.DT_LevelManager` (`self.GameInstance`)) (`KismetStringLibrary.Conv_StringToName` (`KismetStringLibrary.Conv_IntToString` (`/Game/BluePrints/BP_GameInstance.DayCounter` (`self.GameInstance`)))))
    (:`then`
      (set `self.NumberEnemies` (`.NumberEnemies_10_D96D0CAA4E9CBA3D52EC0F9B3133C1C5` (break `/Game/BluePrints/STR_LevelManager` _returnvalue)))
      (set `self.CurrentEnemy` 0)
      (`self.SpawnEnemyKnights`)
      (`self.CheckWinOrLose`))))

(event `SpawnEnemyKnights`
  (bind _returnvalue (`KismetSystemLibrary.K2_SetTimerDelegate` (delegate `SpawnEnemyKnights`) 1.0 true))
  (if (< (`self.CurrentEnemy`) (`self.NumberEnemies`))
    (set `self.CurrentEnemy` (+ (`self.CurrentEnemy`) 1))
    (`|SpawnActorFromClass` "/Game/BluePrints/Units/BP_EnemyKnight.BP_EnemyKnight_C" (`KismetMathLibrary.Conv_VectorToTransform` (`|GetArrayItem` (`self.LocationSpawners`))) "Undefined" "MultiplyWithRoot" null null)
    (else
      (`KismetSystemLibrary.K2_ClearAndInvalidateTimerHandle` _returnvalue))))

(event `CheckWinOrLose`
  (bind _returnvalue (`KismetSystemLibrary.K2_SetTimerDelegate` (delegate `CheckWinOrLose`) 1.0 true))
  (bind _outactors (`GameplayStatics.GetAllActorsWithTag` "Building"))
  (if (== (`KismetArrayLibrary.Array_Length` _outactors) 0)
    (`self.Lose`)
    (`KismetSystemLibrary.K2_ClearAndInvalidateTimerHandle` _returnvalue)
    (else
      (bind _outactors_2 (`GameplayStatics.GetAllActorsWithTag` "Enemy"))
      (if (== (`KismetArrayLibrary.Array_Length` _outactors_2) 0)
        (`self.Win`)
        (`KismetSystemLibrary.K2_ClearAndInvalidateTimerHandle` _returnvalue)))))

(event `Win`
  (`GameplayStatics.PlaySound2D` "/Game/Sounds/Special_Collectible_9-1.Special_Collectible_9-1" 1.0 1.0 0.0 null null)
  (`/Game/BluePrints/UI/WBP_GameControl.NewDay` (`self.WBP_GameControl`))
  (`KismetSystemLibrary.PrintString` (`KismetStringLibrary.Conv_IntToString` (`/Game/BluePrints/BP_GameInstance.NextDayBattle` (`self.GameInstance`))))
  (bind _outactors (`GameplayStatics.GetAllActorsWithTag` "Unit"))
  (for _array_element _outactors
    (`self.K2_DestroyActor` _array_element))
  (bind _returnvalue (`|CreateWidget` "/Game/BluePrints/UI/WBP_Win.WBP_Win_C"))
  (`UserWidget.AddToViewport` _returnvalue 0))

(event `Lose`
  (`GameplayStatics.PlaySound2D` "/Game/Sounds/Magical_Interface_8-1.Magical_Interface_8-1" 1.0 1.0 0.0 null null)
  (`UserWidget.AddToViewport` (`self.WBP_Lose`) 0)
  (`GameplayStatics.SetGamePaused` true))

(fn `SetPhase`
  (params (Phase :type "/Game/BluePrints/Enum_GamePhase Enum" :default "NewEnumerator0")))

(fn `UserConstructionScript`)